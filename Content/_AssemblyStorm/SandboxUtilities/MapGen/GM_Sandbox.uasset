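; GM_Sandbox is a game mode that sets up a sandbox level in place of normal scripted enemy waves.
; Its construction script pushes a disable on scripted waves in the EnemyWaveManager.
; When level generation first completes, it finds the SandboxUtilities actor, sets the sandbox origin to the world origin and calls CreateSandbox, with a Created flag preventing repeats on later passes.
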(event `self.OnLevelGenerationComplete`
  (params (pass :type Integer))
  (`parent.OnLevelGenerationComplete` pass)
  (if (not (`self.Created`))
    (set `self.Created` true)
    (bind _returnvalue (`GameplayStatics.GetActorOfClass` "/Game/_AssemblyStorm/SandboxUtilities/SandboxUtilities.SandboxUtilities_C"))
    (set `/Game/_AssemblyStorm/SandboxUtilities/SandboxUtilities.SandboxOrigin` (0.0 0.0 0.0) _returnvalue)
    (`/Game/_AssemblyStorm/SandboxUtilities/SandboxUtilities.CreateSandbox` _returnvalue)))

(fn `UserConstructionScript`
  (bind _enemywavemanager (`self.EnemyWaveManager`))
  (`parent.UserConstructionScript`)
  (`EnemyWaveManager.PushDisableScriptedWaves` _enemywavemanager _enemywavemanager))