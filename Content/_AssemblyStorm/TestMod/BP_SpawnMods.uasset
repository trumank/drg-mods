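; Mod loader actor that spawns mod init Blueprints on BeginPlay, choosing InitSpacerig_C on the space rig or InitCave_C otherwise.
; Force-rescans /Game/ in the Asset Registry and matches generated Blueprint classes by asset name, so mods are discovered without hard references.
; Each match is loaded synchronously and, unless an instance of that class already exists, spawned with the local FSD player controller as owner.
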(event `self.ReceiveBeginPlay`
  (bind _returnvalue (`FSDGameInstance.GetLocalFSDPlayerController` (`GameFunctionLibrary.GetFSDGameInstance` self)))
  (`AssetRegistry.ScanPathsSynchronous` (`AssetRegistryHelpers.GetAssetRegistry`) (`|MakeArray` "/Game/") true)
  (bind _outassetdata (`AssetRegistry.GetAssets` (`AssetRegistryHelpers.GetAssetRegistry`) (make `ARFilter` :`ClassNames` (`|MakeArray` "BlueprintGeneratedClass" :!type "Name"))))
  (for _array_element _outassetdata
    (if (== (`KismetStringLibrary.Conv_NameToString` (`.AssetName` (break `AssetData` _array_element))) (`KismetMathLibrary.SelectString` "InitSpacerig_C" "InitCave_C" (`FSDPlayerController.IsOnSpaceRig` _returnvalue)))
      (bind _returnvalue_2 (`KismetSystemLibrary.LoadClassAsset_Blocking` (`KismetSystemLibrary.Conv_SoftClassPathToSoftClassRef` (`KismetSystemLibrary.MakeSoftClassPath` (`AssetRegistryHelpers.GetExportTextName` _array_element)))))
      (bind _asactor (castclass `Actor` _returnvalue_2))
      (bind _returnvalue_3 (`GameplayStatics.GetActorOfClass` _asactor))
      (`/Engine/EditorBlueprintResources/StandardMacros.IsValid` _returnvalue_3
        (:`Is Not Valid`
          (`|SpawnActorFromClass` _asactor (`KismetMathLibrary.MakeTransform` (0.0 0.0 0.0)) "AlwaysSpawn" "OverrideRootScale" _returnvalue null))))))

(fn `UserConstructionScript`)