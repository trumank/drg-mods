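; BP_CrystalDummy is a test-mod Blueprint, apparently a crystal stand-in, with debug logging of the world's actors.
; Its construction script sets a stretched actor scale, calls the empty DoStuff event, then runs the parent script.
; The Timer event logs the level name plus every actor's name and location through a log state.
; The looping timer and TestModState lookup that would drive that logging are disconnected and never run.
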(event `DoStuff`)

(event `Timer`
  (bind _aslog_state (`self.AsLog State`))
  (`/Game/_AssemblyStorm/TestMod/TestModState.LogMessage` _aslog_state "We're here")
  (bind _returnvalue (`GameplayStatics.GetCurrentLevelName` true))
  (`/Game/_AssemblyStorm/TestMod/TestModState.LogMessage` _aslog_state _returnvalue)
  (bind _outactors (`GameplayStatics.GetAllActorsOfClass` "/Script/Engine.Actor"))
  (`/Game/_AssemblyStorm/TestMod/TestModState.LogMessage` _aslog_state (`KismetStringLibrary.Concat_StrStr` "Found " (`KismetStringLibrary.Conv_IntToString` (`KismetArrayLibrary.Array_Length` _outactors)) " actors"))
  (for _array_element _outactors
    (`/Game/_AssemblyStorm/TestMod/TestModState.LogMessage` _aslog_state (`KismetStringLibrary.Concat_StrStr` "Actor: " (`KismetSystemLibrary.GetDisplayName` _array_element) " location: " (`KismetStringLibrary.Conv_VectorToString` (`self.K2_GetActorLocation` _array_element))))))

(fn `UserConstructionScript`
  (`self.SetActorScale3D` (2.0 1.0 2.0))
  (`self.DoStuff`)
  (`parent.UserConstructionScript`))